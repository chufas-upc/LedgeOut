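; Lobby player controller that drives the main menu UI and switches between menu and lobby cameras.
; On BeginPlay, only the primary local player creates the main menu widget, binds to online session connection changes and sets Game-and-UI input so debug keys work.
; Disconnected switches to the menu camera, while Host and Client both switch to the lobby camera.
; A debug T key creates an additional local player.
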(event Custom|ConnectionChanged
  (params (SessionType :type ELobbyStatus%20Enum :default "Disconnected"))
  (switch Utilities|FlowControl|Switch|SwitchonELobbyStatus SessionType
    (:Disconnected
      (Class|LobbyPlayerController|SwitchtoMenuCamera))
    (:Host
      (Class|LobbyPlayerController|SwitchtoLobbyCamera :!label _label))
    (:Client
      (goto _label))))

(event EventBeginPlay
  (if (and (Pawn|IsLocalPlayerController) (Class|PlayerController|IsPrimaryPlayer))
    (bind _returnvalue (UserInterface|CreateWidget "/Game/Blueprints/Widgets/WBP_MainMenuWidget.WBP_MainMenuWidget_C" self))
    (bind _output_get (Variables|Default|SetMenuWidget _returnvalue))
    (UserInterface|Viewport|AddtoViewport _output_get 0)
    (EventDispatchers|BindEventtoOnConnectionChanged (Subsystems|GetOnlineSessionsSubsystem) (delegate Custom|ConnectionChanged))
    (Input|SetInputModeGameandUI self 0 "DoNotLock" false true) ; Necesario para poder pulsar DebugKeys
  ))

(event Input|KeyboardEvents|DebugKeyT
  (params (Key :type Key%20Structure :default "None") (ActionValue :type Input%20Action%20Value%20Structure))
  (:Pressed
    (Class|GameplayStatics|CreatePlayer -1)))

(fn ConstructionScript)