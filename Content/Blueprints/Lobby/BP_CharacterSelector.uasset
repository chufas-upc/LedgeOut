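; BP_CharacterSelector is a lobby slot actor that displays the occupying player's name and selected character.
; On slot state changes it calls the parent handler, then updates the text render from the player data.
; It async-loads the first skin of the selected character from BP_MenuGameMode's AvailableCharacters, hiding the mesh until the load completes.
; A per-selector stand material preview sits unconnected in the construction script.
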(event `self.ReceiveBeginPlay`
  (bind _asbp_menu_game_mode (cast `/Game/Blueprints/Lobby/BP_MenuGameMode` (`GameplayStatics.GetGameMode`)))
  (set `self.As BP Menu Game Mode` _asbp_menu_game_mode))

(event `self.OnSlotOccupiedStateChanged`
  (params (bOccupied :type Boolean) (OccupyingPlayerData :type "LobbyPlayerData Structure (by ref)"))
  (bind (_playername _localplayerindex _selectedcharacterindex) (break `LobbyPlayerData` OccupyingPlayerData))
  (bind _textrender (`self.TextRender`))
  (bind _charactermesh (`self.CharacterMesh`))
  (bind _availablecharacters (`/Game/Blueprints/Lobby/BP_MenuGameMode.AvailableCharacters` (`self.As BP Menu Game Mode`)))
  (`parent.OnSlotOccupiedStateChanged` bOccupied OccupyingPlayerData)
  (`|ExecutionSequence`
    (:`then_0`
      (`TextRenderComponent.K2_SetText` _textrender (`KismetTextLibrary.Conv_StringToText` _playername))
      (`SceneComponent.SetVisibility` _textrender true false))
    (:`then_1`
      (if (`KismetArrayLibrary.Array_IsValidIndex` _availablecharacters _selectedcharacterindex)
        (`SceneComponent.SetVisibility` (`self.CharacterMesh`) false false)
        (bind _object (`|LoadAsset` (`|GetArrayItem` (`.Skins_8_5D907F674CF7EA7F96010E83FD2DE80D` (break `/Game/Blueprints/S_CharacterData` (`|GetArrayItem` _availablecharacters _selectedcharacterindex)))))
          (:`Completed`
            (bind _asskeletal_mesh (cast `SkeletalMesh` _object))
            (`SceneComponent.SetVisibility` _charactermesh true false)
            (`SkeletalMeshComponent.SetSkeletalMeshAsset` _charactermesh _asskeletal_mesh)))))))

(fn `UserConstructionScript`)