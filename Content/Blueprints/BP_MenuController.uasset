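; Player controller for the main menu that shows the menu widget to the primary local player and follows online connection state.
; On BeginPlay it binds to the OnlineSessionsSubsystem connection event, switching to the lobby camera for host or client and the menu camera when disconnected.
; Debug keys force the lobby camera, create a LAN session and host beacon, and trigger server or hardcoded-IP client travel to the game map.
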(event Custom|ConnectionChanged
  (params (SessionType :type ELobbyStatus%20Enum :default "Disconnected"))
  (switch Utilities|FlowControl|Switch|SwitchonELobbyStatus SessionType
    (:Disconnected
      (Class|LobbyPlayerController|SwitchtoMenuCamera))
    (:Host
      (Class|LobbyPlayerController|SwitchtoLobbyCamera :!label _label))
    (:Client
      (goto _label))))

(event EventBeginPlay
  (if (and (Pawn|IsLocalPlayerController) (Class|PlayerController|IsPrimaryPlayer))
    (bind _returnvalue (UserInterface|CreateWidget "/Game/Blueprints/Widgets/WBP_MainMenuWidget.WBP_MainMenuWidget_C" self))
    (bind _output_get (Variables|Default|SetMenuWidget _returnvalue))
    (UserInterface|Viewport|AddtoViewport _output_get 0)
    (EventDispatchers|BindEventtoOnConnectionChanged (Subsystems|GetOnlineSessionsSubsystem) (delegate Custom|ConnectionChanged))
    (Input|SetInputModeGameandUI self 0 "DoNotLock" false true) ; Necesario para poder pulsar DebugKeys
  ))

(event Input|KeyboardEvents|DebugKeyX
  (params (Key :type Key%20Structure :default "None") (ActionValue :type Input%20Action%20Value%20Structure))
  (:Pressed
    (Class|LobbyPlayerController|SwitchtoLobbyCamera)))

(event Input|KeyboardEvents|DebugKeyC
  (params (Key :type Key%20Structure :default "None") (ActionValue :type Input%20Action%20Value%20Structure))
  (:Pressed
    (Class|OnlineSessionsSubsystem|ClientTravel (Subsystems|GetOnlineSessionsSubsystem) self "192.168.1.5/Game/Maps/L_Game" "TRAVEL_Absolute" false)))

(event Input|KeyboardEvents|DebugKeyV
  (params (Key :type Key%20Structure :default "None") (ActionValue :type Input%20Action%20Value%20Structure))
  (:Pressed
    (|Session self 4 true false
      (:OnSuccess
        (Development|PrintString "Session creada!"))
      (:OnFailure
        _))
    (Development|PrintString (Utilities|String|SelectString "Conexión exitosa" "Conexión fallida" false))
    (Class|OnlineSessionsSubsystem|ForceCreateHostBeacon (Subsystems|GetOnlineSessionsSubsystem))))

(event Input|KeyboardEvents|DebugKeyB
  (params (Key :type Key%20Structure :default "None") (ActionValue :type Input%20Action%20Value%20Structure))
  (:Pressed
    (Development|PrintString "Intentando Server Travel")
    (Class|OnlineSessionsSubsystem|ServerTravel (Subsystems|GetOnlineSessionsSubsystem) "/Game/Maps/L_Game?listen" false)))

(fn ConstructionScript)